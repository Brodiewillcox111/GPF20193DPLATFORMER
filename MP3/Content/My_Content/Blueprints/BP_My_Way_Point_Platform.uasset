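; Waypoint-driven moving platform actor with a configurable mesh and material, optional looping, and Start and Stop functions.
; BeginPlay hides the waypoint actors and calls the platform start inside that loop, resetting to the first pair and playing a rate-scaled timeline.
; The timeline lerps actor location between waypoint pairs; its event advances indices or restarts the path when looping.
; SetPosition assigns the current index's location to NextWaypointPosition and vice versa.
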(event `self.ReceiveBeginPlay`
  (for _array_element (`self.Waypoints`)
    (`self.SetActorHiddenInGame` _array_element true)
    (`self.Platform_Start`)))

(event `Platform_Start`
  (bind _motion_timeline (`self.Motion_Timeline`))
  (`self.Set_First_Waypoint`)
  (`TimelineComponent.SetPlayRate` _motion_timeline (`self.Rate`))
  (`TimelineComponent.PlayFromStart` _motion_timeline))

(fn `Path_Is_Finished`
  (returns (Is_Finished :type Boolean))
  (return (== (`self.Next_Way_Point_Index`) (- (`KismetArrayLibrary.Array_Length` (`self.Waypoints`)) 1))))

(fn `Set_First_Waypoint`
  (set `self.Current_Waypoint_Index` 0)
  (set `self.Next_Way_Point_Index` 1)
  (`self.Set_Position`))

(fn `Set_Next_Waypoint`
  (bind _result (`/Engine/EditorBlueprintResources/StandardMacros.IncrementInt` (`self.Current_Waypoint_Index`))
    (:`  `
      (set `self.Next_Way_Point_Index` (+ _result 1))
      (`self.Set_Position`))))

(fn `Set_Position`
  (bind _waypoints (`self.Waypoints`))
  (set `self.Next_Waypoint_Position` (`self.K2_GetActorLocation` (`|GetArrayItem` _waypoints (`self.Current_Waypoint_Index`))))
  (set `self.Current_Waypoint_Position` (`self.K2_GetActorLocation` (`|GetArrayItem` _waypoints (`self.Next_Way_Point_Index`)))))

(fn `Start`
  (`self.Platform_Start`))

(fn `stop`
  (`TimelineComponent.Stop` (`self.Motion_Timeline`)))

(fn `UserConstructionScript`
  (bind _platform_mesh (`self.Platform Mesh`))
  (`StaticMeshComponent.SetStaticMesh` _platform_mesh (`self.Static_Mesh`))
  (`PrimitiveComponent.SetMaterial` _platform_mesh 0 (`self.Material`)))